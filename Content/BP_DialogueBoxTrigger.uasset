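; BP_DialogueBoxTrigger is a placeable trigger volume that shows a dialogue box when the side-scroller player character walks into it.
; On the first Box overlap it creates a WBP_DialogueBox, fills in the speaker name, text and dialogue length, adds it to the viewport and destroys itself.
; The DoOnce runs before the class check, so an overlap by any other actor uses up the trigger.
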(event `self.Box.OnComponentBeginOverlap`
  (params (OverlappedComponent :type "PrimitiveComponent Object Reference") (OtherActor :type "Actor Object Reference") (OtherComp :type "PrimitiveComponent Object Reference") (OtherBodyIndex :type Integer) (bFromSweep :type Boolean) (SweepResult :type "HitResult Structure (by ref)"))
  (`/Engine/EditorBlueprintResources/StandardMacros.DoOnce` false
    (:`Completed`
      (if (== (`GameplayStatics.GetObjectClass` OtherActor) "/Game/2DSideScroller/Blueprints/BP_SideScrollerCharacter.BP_SideScrollerCharacter_C")
        (bind _returnvalue (`|CreateWidget` "/Game/WBP_DialogueBox.WBP_DialogueBox_C"))
        (set `TextBlock.Text` (`self.SpeakerName`) (`/Game/WBP_DialogueBox.SpeakerName` _returnvalue))
        (set `TextBlock.Text` (`self.SpeakerText`) (`/Game/WBP_DialogueBox.SpeakerText` _returnvalue))
        (set `/Game/WBP_DialogueBox.DialogueLength` (`self.DialogueLength`) _returnvalue)
        (`UserWidget.AddToViewport` _returnvalue 0)
        (`self.K2_DestroyActor`)))))

(fn `UserConstructionScript`)